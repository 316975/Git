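; Projectile bullet actor that deals damage between the first-person player character and the BP_Monolith, destroying itself after two seconds or on bounce.
; BeginPlay caches references to both actors, and the sphere overlap compares the other actor against them.
; As wired, overlapping the monolith damages the player and overlapping the player damages the monolith, opposite to the actor touched.
; DoOnce gates each hit and debug print, then the bullet is destroyed after a short delay.
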(event OnComponentBeginOverlap(Sphere)
  (params (OverlappedComponent :type Primitive%20Component%20Object%20Reference) (OtherActor :type Actor%20Object%20Reference) (OtherComp :type Primitive%20Component%20Object%20Reference) (OtherBodyIndex :type Integer) (bFromSweep :type Boolean) (SweepResult :type Hit%20Result%20Structure%20%28by%20ref%29))
  (bind _characterref (Variables|Default|GetcharacterRef))
  (bind _monolithref (Variables|Default|GetmonolithRef))
  (if (== (Variables|Default|GetmonolithRef) OtherActor)
    ;[0.15 0.15 0.15 0.5] player hit
    (Utilities|FlowControl|DoOnce false
      (:Completed
        (Default|TakeDamage _characterref (Variables|Default|GetbulletDamage))
        (Development|PrintString (Utilities|String|ToString(Text) (Utilities|Text|FormatText "{ } hit" _characterref)) true true "(R=1.000000,G=0.502887,B=1.000000,A=1.000000)")))
    (else
      ;[0.15 0.15 0.15 0.5] monolith hit
      (if (== OtherActor (Variables|Default|GetcharacterRef))
        (Utilities|FlowControl|DoOnce false
          (:Completed
            (Default|TakeDamage _monolithref (Variables|Default|GetbulletDamage))
            (Development|PrintString (Utilities|String|ToString(Text) (Utilities|Text|FormatText "{ } hit" _monolithref)) true true "(R=1.000000,G=0.502887,B=1.000000,A=1.000000)")))
        (else
          ;[0.15 0.15 0.15 0.5] invalid hit
          (Utilities|FlowControl|DoOnce false
            (:Completed
              (Development|PrintString (Utilities|String|ToString(Text) (Utilities|Text|FormatText "{ } hit" OtherActor)) true true "(R=1.000000,G=0.502887,B=1.000000,A=1.000000)")))))))
  (Utilities|FlowControl|Delay 0.5)
  (Actor|DestroyActor))

(event OnProjectileBounce(ProjectileMovement)
  (params (ImpactResult :type Hit%20Result%20Structure%20%28by%20ref%29) (ImpactVelocity :type Vector%20%28by%20ref%29 :default "0, 0, 0"))
  (Development|PrintString "projectile bounce")
  (Actor|DestroyActor))

(event Custom|Destroy%20Actor
  ;[0.15 0.15 0.15 0.5] init
  (Actor|DestroyActor))

(event Collision|EventActorBeginOverlap
  (params (OtherActor :type Actor%20Object%20Reference)))

(event EventTick
  (params (DeltaSeconds :type Float%20%28single-precision%29)))

(event EventBeginPlay
  ;[0.15 0.15 0.15 0.5] init
  (Utilities|Time|SetTimerbyEvent (delegate Custom|Destroy%20Actor) 2.0)
  (bind _asbp_first_person_character (Utilities|Casting|CastToBP_FirstPersonCharacter (Game|GetPlayerCharacter 0)))
  (Variables|Default|SetcharacterRef _asbp_first_person_character)
  (bind _returnvalue (Actor|GetActorOfClass "/Game/Blueprints/BP_Monolith.BP_Monolith_C"))
  (Variables|Default|SetmonolithRef _returnvalue))

(fn ConstructionScript)