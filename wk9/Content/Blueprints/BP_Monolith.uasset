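; BP_Monolith is a damageable monolith that triggers GameOver on the first-person game mode when its health runs out.
; Shot forwards damage to takeDamage, where a DoOnce gate subtracts health and turns the cylinder and two cones glowing red.
; If health remains, a half-second delay restores the white glow and reopens the gate, so hits during the flash are ignored.
; At zero health it stays red and the gate stays closed.
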(event Custom|takeDamage
  (params (damageValue :type Float%20%28double-precision%29))
  (Utilities|FlowControl|DoOnce false :!label _label
    (:Completed
      (Variables|Default|SettakingDamage true)
      (Rendering|Material|SetMaterial (Variables|Default|GetCylinder) 0 "/Game/Assets/M_GlowRed.M_GlowRed")
      (bind _output_get (Variables|Default|SetcurrentHealth (- (Variables|Default|GetcurrentHealth) damageValue)))
      (if (<= _output_get 0.0)
        (Default|GameOver (Variables|Default|GetgameModeRef))
        (else
          (Utilities|FlowControl|Delay 0.5)
          (Rendering|Material|SetMaterial (Variables|Default|GetCylinder) 0 "/Game/Assets/M_GlowWhite.M_GlowWhite")
          (Variables|Default|SettakingDamage false)
          (goto _label Reset))))))

(event EventShot
  (params (damageValue :type Float%20%28double-precision%29))
  (CallFunction|TakeDamage damageValue))

(event Collision|EventActorBeginOverlap
  (params (OtherActor :type Actor%20Object%20Reference)))

(event EventTick
  (params (DeltaSeconds :type Float%20%28single-precision%29)))

(event EventBeginPlay
  (bind _asbp_first_person_game_mode (Utilities|Casting|CastToBP_FirstPersonGameMode (Game|GetGameMode)))
  (Variables|Default|SetgameModeRef _asbp_first_person_game_mode))

(fn ConstructionScript)