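; Large hostile enemy with a billboarded Paper sprite that pursues either the player or the Monolith.
; It starts toward the Monolith, then a delayed Tick rechecks which is closer and uses AI Move To toward random reachable points nearby.
; Being shot redirects it to the player, flashes it red and drains health until destroyed.
; Its collision turns off while the player slides; the attack event is an empty stub.
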(event OnComponentBeginOverlap(CapsuleComponent)
  (params (OverlappedComponent :type Primitive%20Component%20Object%20Reference) (OtherActor :type Actor%20Object%20Reference) (OtherComp :type Primitive%20Component%20Object%20Reference) (OtherBodyIndex :type Integer) (bFromSweep :type Boolean) (SweepResult :type Hit%20Result%20Structure%20%28by%20ref%29))
  ;[0.15 0.15 0.15 0.5] collision based movement
  (if (== OtherActor "/Game/FirstPerson/Blueprints/BP_FirstPersonCharacter.BP_FirstPersonCharacter")
    (Variables|Default|SetcurrentTarget (Variables|Default|GetplayerRef))
    (Development|PrintString "collision target player" true true "(R=1.000000,G=0.000000,B=1.000000,A=1.000000)")
    (elif (== OtherActor "/Game/Blueprints/BP_Monolith.BP_Monolith")
      (Variables|Default|SetcurrentTarget (Variables|Default|GetmonolithRef))
      (Development|PrintString "collision target monolith" true true "(R=1.000000,G=0.000000,B=1.000000,A=1.000000)"))))

(event OnComponentEndOverlap(CapsuleComponent)
  (params (OverlappedComponent :type Primitive%20Component%20Object%20Reference) (OtherActor :type Actor%20Object%20Reference) (OtherComp :type Primitive%20Component%20Object%20Reference) (OtherBodyIndex :type Integer))
  ;[0.15 0.15 0.15 0.5] collision based movement
)

(event Custom|moveToPlayer
  (bind _playerref (Variables|Default|GetplayerRef))
  (bind _charactermovement (Variables|Character|GetCharacterMovement))
  ;[0.15 0.15 0.15 0.5] movement to player
  (Class|NavMovementInterface|StopActiveMovement _charactermovement)
  (Components|Movement|StopMovementImmediately _charactermovement)
  (Variables|Default|SetcurrentTarget _playerref)
  (AI|AIMoveTo self (.RandomLocation (AI|Navigation|GetRandomReachablePointinRadius (Transformation|GetWorldLocation (Variables|/Script/Engine.Character|GetCapsuleComponent _playerref)) 5e+02 0 0)) 0 5.0 false
    (:then
      (Development|PrintString "movement player" true true "(R=1.000000,G=0.000000,B=1.000000,A=1.000000)"))))

(event Custom|faceCamera
  ;[0.15 0.15 0.15 0.5] sprite face camera
  (Transformation|SetActorRotation (Math|Rotator|FindLookatRotation (Transformation|GetActorLocation) (Transformation|GetActorLocation (Game|GetPlayerCharacter 0)))))

(event Custom|removeCollision
  (bind _capsulecomponent (Variables|Collision|GetCapsuleComponent))
  ;[0.15 0.15 0.15 0.5] remove collision when player is sliding
  (if (Variables|/Game/FirstPerson/Blueprints/BP_FirstPersonCharacter.BP_FirstPersonCharacter_C|GetisSliding (Variables|Default|GetplayerRef))
    (Collision|SetCollisionEnabled _capsulecomponent "NoCollision")
    (else
      (Collision|SetCollisionEnabled _capsulecomponent "QueryAndPhysics"))))

(event Custom|moveToMonolith
  (bind _monolithref (Variables|Default|GetmonolithRef))
  (bind _charactermovement (Variables|Character|GetCharacterMovement))
  ;[0.15 0.15 0.15 0.5] movement to monolith
  (Class|NavMovementInterface|StopActiveMovement _charactermovement)
  (Components|Movement|StopMovementImmediately _charactermovement)
  (Variables|Default|SetcurrentTarget _monolithref)
  (AI|AIMoveTo self (.RandomLocation (AI|Navigation|GetRandomReachablePointinRadius (Transformation|GetWorldLocation (Variables|/Game/Blueprints/BP_Monolith.BP_Monolith_C|GetenemyHit _monolithref)) 5e+02 0 0)) 0 5.0 false
    (:then
      (Development|PrintString "movement monolith" true true "(R=1.000000,G=0.000000,B=1.000000,A=1.000000)"))))

(event Custom|distanceCheck
  ;[0.15 0.15 0.15 0.5] distance based movement
  (if (> (Transformation|GetDistanceTo (Variables|Default|GetmonolithRef)) (Transformation|GetDistanceTo (Variables|Default|GetplayerRef)))
    (CallFunction|MovetoPlayer)
    (else
      (CallFunction|MovetoMonolith))))

(event Custom|attack
  ;[0.15 0.15 0.15 0.5] attack system
  (if (not (== (Variables|Default|GetcurrentTarget) (Variables|Default|GetplayerRef)))
    (if (== (Variables|Default|GetcurrentTarget) (Variables|Default|GetmonolithRef))
      _)))

(event EventBeginPlay
  ;[0.15 0.15 0.15 0.5] init
  (bind _asbp_first_person_character (Utilities|Casting|CastToBP_FirstPersonCharacter (Game|GetPlayerCharacter 0)))
  (Variables|Default|SetplayerRef _asbp_first_person_character)
  (bind _returnvalue (Actor|GetActorOfClass "/Game/Blueprints/BP_Monolith.BP_Monolith_C"))
  (Variables|Default|SetmonolithRef _returnvalue)
  (CallFunction|MovetoMonolith))

(event EventTick
  (params (DeltaSeconds :type Float%20%28single-precision%29))
  ;[1 0.5903 0] timer
  (CallFunction|FaceCamera)
  (Utilities|FlowControl|Delay 2.5)
  (CallFunction|DistanceCheck)
  (CallFunction|RemoveCollision))

(event EventShot
  (bind _papersprite (Variables|Default|GetPaperSprite))
  ;[0.15 0.15 0.15 0.5] hit behaviour
  (CallFunction|MovetoPlayer)
  (Sprite|SetSpriteColor _papersprite "(R=1.000000,G=0.000000,B=0.000000,A=1.000000)")
  (Utilities|FlowControl|Delay 0.2)
  (Sprite|SetSpriteColor _papersprite "(R=1.000000,G=1.000000,B=1.000000,A=1.000000)")
  (bind _result (Math|Float|DecrementFloat (Variables|Default|GetHealth))
    (:%20%20
      (if (<= _result 0.0)
        (Actor|DestroyActor)
        (Default|CallOnDestroyed)))))

(fn ConstructionScript)