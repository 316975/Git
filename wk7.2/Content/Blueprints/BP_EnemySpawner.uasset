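; BP_EnemySpawner is an actor that spawns queued enemy classes at its own transform.
; A looping one-second timer pops the front of EnemyQueue and spawns it, binding an event to the enemy's destruction.
; AddEnemyToQueue appends classes; its SphereCollision overlap check leads to no action.
; A defeat event forwards OnEnemyDefeated to BP_FirstPersonGameMode.
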(event Custom|tryToSpawn
  (CallFunction|SpawnEnemy))

(event Custom|onEnemyDefeated
  (bind _asbp_first_person_game_mode (Utilities|Casting|CastToBP_FirstPersonGameMode (Game|GetGameMode)))
  (Default|OnEnemyDefeated _asbp_first_person_game_mode))

(event EventBeginPlay
  (Utilities|Time|SetTimerbyEvent (delegate Custom|tryToSpawn) 1.0 true))

(fn ConstructionScript)

(fn SpawnEnemy
  (if (Utilities|Array|IsValidIndex (Variables|Default|GetenemyQueue))
    (bind _returnvalue (Game|SpawnActorfromClass (Utilities|Array|Get(acopy) (Variables|Default|GetenemyQueue)) (Transformation|GetActorTransform) "Undefined" "MultiplyWithRoot" 0 0))
    (EventDispatchers|BindEventtoOnDestroyed _returnvalue (EventDispatchers|CreateEvent :!event Custom|onEnemyDefeated))
    (Utilities|Array|RemoveIndex (Variables|Default|GetenemyQueue))
    (return true)
    (else
      (return false))))

(fn AddEnemytoQueue
  (params (EnemyClass :type BP%20Hostile%20Class%20Reference%20%28by%20ref%29))
  (Utilities|Array|Add (Variables|Default|GetenemyQueue) EnemyClass)
  (if (Utilities|Array|IsValidIndex (Collision|GetOverlappingActors (Variables|Default|GetsphereCollision) 0 :!class /Script/Engine.PrimitiveComponent))
    _))