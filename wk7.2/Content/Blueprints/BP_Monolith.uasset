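; BP_Monolith is an actor with a health value that flashes red when hit.
; The takeDamage event swaps the cylinder and two cones to a red glow material and subtracts health, restoring white after half a second.
; At zero health or below it stays red and flagged as taking damage.
; BeginPlay loops a zero-damage hit every 2.5 seconds, so it pulses red without losing health.
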(event Custom|takeDamage
  (params (damageValue :type Float%20%28double-precision%29))
  (Variables|Default|SettakingDamage true)
  (Rendering|Material|SetMaterial (Variables|Default|GetCylinder) 0 "/Game/Assets/M_GlowRed.M_GlowRed")
  (bind _output_get (Variables|Default|Sethealth (- (Variables|Default|Gethealth) damageValue)))
  (if (not (<= _output_get 0.0))
    (Utilities|FlowControl|Delay 0.5)
    (Rendering|Material|SetMaterial (Variables|Default|GetCylinder) 0 "/Game/Assets/M_GlowWhite.M_GlowWhite")
    (Variables|Default|SettakingDamage false)))

(event Collision|EventActorBeginOverlap
  (params (OtherActor :type Actor%20Object%20Reference)))

(event EventTick
  (params (DeltaSeconds :type Float%20%28single-precision%29)))

(event EventBeginPlay
  (CallFunction|TakeDamage 0.0 :!label _label)
  (Utilities|FlowControl|Delay 2.5)
  (goto _label))

(fn ConstructionScript)